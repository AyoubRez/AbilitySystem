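; BP_Player is the player character Blueprint that reflects health and mana changes in the UI.
; OnHealthChange and OnManaChange convert values to a current-over-max ratio and push it to glass ball widgets in the player controller's PrimaryUI.
; Health changes also update the HealthBar widget held by the character's own HealthBar component.
; BeginPlay, overlap and Tick are disabled stubs, so all logic here is event-driven.
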(event EventBeginPlay
  (|CallParentFunction) ; This node is disabled and will not be called.\nDrag off pins to build functionality.
)

(event Collision|EventActorBeginOverlap
  (params (OtherActor :type Actor%20Object%20Reference))
  (|CallParentFunction OtherActor) ; This node is disabled and will not be called.\nDrag off pins to build functionality.
)

(event EventTick
  (params (DeltaSeconds :type Float%20%28single-precision%29))
  (|CallParentFunction DeltaSeconds) ; This node is disabled and will not be called.\nDrag off pins to build functionality.
)

(event EventOnHealthChange
  (params (Health :type Float%20%28single-precision%29) (MaxHealth :type Float%20%28single-precision%29))
  (bind _returnvalue (/ Health MaxHealth))
  (bind _asbp_player_controller_base (Utilities|Casting|CastToBP_PlayerControllerBase (Pawn|GetController)))
  (Default|SetPercentage (Variables|/Game/_Game/UI/PrimaryUI.PrimaryUI_C|GetHealthGlassBall (Variables|/Game/_Game/Gameplay/BP_PlayerControllerBase.BP_PlayerControllerBase_C|GetPrimaryUI _asbp_player_controller_base)) _returnvalue)
  (bind _ashealth_bar (Utilities|Casting|CastToHealthBar (UserInterface|GetUserWidgetObject (Variables|Default|GetHealthBar))))
  (Default|SetPercentage _ashealth_bar _returnvalue))

(event EventOnManaChange
  (params (Mana :type Float%20%28single-precision%29) (MaxMana :type Float%20%28single-precision%29))
  (bind _asbp_player_controller_base (Utilities|Casting|CastToBP_PlayerControllerBase (Pawn|GetController)))
  (Default|SetPercentage (Variables|/Game/_Game/UI/PrimaryUI.PrimaryUI_C|GetManaGlassBall (Variables|/Game/_Game/Gameplay/BP_PlayerControllerBase.BP_PlayerControllerBase_C|GetPrimaryUI _asbp_player_controller_base)) (/ Mana MaxMana)))

(fn ConstructionScript
  (|CallParentFunction))