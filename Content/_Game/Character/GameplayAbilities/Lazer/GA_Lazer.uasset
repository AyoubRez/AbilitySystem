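; Gameplay ability for a laser skill that fires a beam from the character, damaging and knocking back targets.
; Activation commits cost and cooldown, plays the casting montage, then after a short delay attaches BP_BeamLazer to a mesh socket and enables camera-controlled rotation.
; Damage gameplay events supply target data for the damage effect and a stunning push away from the beam's end.
; Ending removes mana-drain effects, destroys the beam and restores rotation.
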(event Ability|EventActivateAbility
  (|CallParentFunction)
  (Ability|CommitAbility)
  (CallFunction|DoUiCooldown)
  (|PlayMontageandWaitProxy "None" "/Game/_Game/Character/Animations/AnimMontage/AM_LazerCasting.AM_LazerCasting" 1.0 "Start" true 1.0 0.0
    (:then
      (Utilities|FlowControl|Delay 0.3)
      (bind _characterbase (CallFunction|GetPlayerInfo))
      (bind _spawnedactor (|SpawnActor :Class "/Game/_Game/Character/GameplayAbilities/Lazer/BP_BeamLazer.BP_BeamLazer_C" :Instigator _characterbase)
        (:then
          (bind _output_get (Variables|Default|SetLazerActor _spawnedactor))
          (Transformation|AttachComponentToComponent _output_get (Variables|/Script/Engine.Character|GetMesh _characterbase) "lazer" "SnapToTarget" "SnapToTarget" "KeepRelative" true)
          (Default|MakeCameraControlRotation _characterbase true)
          (bind _payload (Ability|Tasks|WaitGameplayEvent "(TagName=\"skill.lazer.dealdamage\")" 0)
            (:EventReceived
              (GameplayEffects|ApplyGameplayEffectToTarget (.TargetData (Utilities|Struct|BreakGameplayEventData _payload)) "/Game/_Game/Character/GameplayAbilities/Lazer/GE_LazerDamage.GE_LazerDamage_C" 1 1)
              (for _array_element (Ability|TargetData|GetActorsfromTargetData (.TargetData (Utilities|Struct|BreakGameplayEventData _payload)))
                (bind _asbp_character_base (Utilities|Casting|CastToBP_CharacterBase _array_element))
                (Default|PushCharacter _asbp_character_base (Math|Vector|Normalize (- (Transformation|GetActorLocation _asbp_character_base) (Transformation|GetWorldLocation (Variables|/Game/_Game/Character/GameplayAbilities/Lazer/BP_BeamLazer.BP_BeamLazer_C|GetLazerEndDetector (.AsBP%20Beam%20Lazer (Utilities|Casting|CastToBP_BeamLazer (Variables|Default|GetLazerActor))))))) 5e+02 0.3)))))))))

(event Ability|EventOnEndAbility
  (params (bWasCancelled :type Boolean))
  (|CallParentFunction bWasCancelled)
  (Ability|RemoveGameplayEffectFromOwnerWithAssetTags "(GameplayTags=((TagName=\"skill.lazer.drainingmana\")))")
  (Actor|DestroyActor (Variables|Default|GetLazerActor))
  (bind _characterbase (CallFunction|GetPlayerInfo))
  (Default|MakeCameraControlRotation _characterbase false))