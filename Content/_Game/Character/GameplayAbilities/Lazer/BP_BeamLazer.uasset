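; BP_BeamLazer is the laser beam actor for a gameplay ability, damaging hostile characters at the beam's end.
; Each tick it offsets the beam mesh's end bone through LazerBeamAnimBp, stretching the beam to LazerEndDetector.
; The detector's overlaps track characters hostile to the instigator.
; A looping timer sends them as target data in a Skill.lazer.dealdamage gameplay event to the instigator, leaving damage to the receiver.
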(event OnComponentBeginOverlap(LazerEndDetector)
  (params (OverlappedComponent :type Primitive%20Component%20Object%20Reference) (OtherActor :type Actor%20Object%20Reference) (OtherComp :type Primitive%20Component%20Object%20Reference) (OtherBodyIndex :type Integer) (bFromSweep :type Boolean) (SweepResult :type Hit%20Result%20Structure%20%28by%20ref%29))
  (bind _asbp_character_base (Utilities|Casting|CastToBP_CharacterBase OtherActor))
  (bind _asbp_character_base_2 (Utilities|Casting|CastToBP_CharacterBase (Game|GetInstigator)))
  (bind _returnvalue (Class|CharacterBase|IsOtherHostile _asbp_character_base_2 _asbp_character_base))
  (if _returnvalue
    (Utilities|Array|AddUnique (Variables|Default|GetOverlappingActors) _asbp_character_base)))

(event OnComponentEndOverlap(LazerEndDetector)
  (params (OverlappedComponent :type Primitive%20Component%20Object%20Reference) (OtherActor :type Actor%20Object%20Reference) (OtherComp :type Primitive%20Component%20Object%20Reference) (OtherBodyIndex :type Integer))
  (bind _asbp_character_base (Utilities|Casting|CastToBP_CharacterBase OtherActor))
  (Utilities|Array|RemoveItem (Variables|Default|GetOverlappingActors) _asbp_character_base))

(event Custom|SendDealDamageEvent
  ;[1 1 1] Send Damage event
  (if (Math|Conversions|ToBoolean(Integer) (Utilities|Array|Length (Variables|Default|GetOverlappingActors)))
    (Ability|SendGameplayEventtoActor (Game|GetInstigator) "(TagName=\"skill.lazer.dealdamage\")" (Utilities|Struct|MakeGameplayEventData "(TagName=\"\")" 0 0 0 0 "()" "(GameplayTags=)" "(GameplayTags=)" 0.0 (Ability|TargetData|AbilityTargetDatafromActorArray (Variables|Default|GetOverlappingActors))))))

(event EventBeginPlay
  (Variables|Default|SetBeamOriginalLength (Math|Vector|VectorLength (- (Transformation|GetSocketLocation (Variables|Default|GetLazeMesh) "end") (Transformation|GetActorLocation))))
  (Utilities|Time|SetTimerbyEvent (delegate Custom|SendDealDamageEvent) 0.3 true))

(event Collision|EventActorBeginOverlap
  (params (OtherActor :type Actor%20Object%20Reference)))

(event EventTick
  (params (DeltaSeconds :type Float%20%28single-precision%29))
  (bind _aslazer_beam_anim_bp (Utilities|Casting|CastToLazerBeamAnimBp (Components|SkeletalMesh|GetAnimInstance (Variables|Default|GetLazeMesh))))
  (Variables|/Game/_Game/Character/GameplayAbilities/Lazer/LazerAssets/LazerBeamAnimBp.LazerBeamAnimBp_C|SetEndBoneOffset _aslazer_beam_anim_bp (Math|Vector|MakeVector (- (Math|Vector|VectorLength (- (Transformation|GetWorldLocation (Variables|Default|GetLazerEndDetector)) (Transformation|GetActorLocation))) (Variables|Default|GetBeamOriginalLength)) 0.0 0.0)))

(fn ConstructionScript)