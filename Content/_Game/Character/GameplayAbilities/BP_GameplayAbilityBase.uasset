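; Base Gameplay Ability Blueprint providing shared helpers for character abilities; its activate and end events are unimplemented.
; GetPlayerInfo casts the owning actor and its controller to the base character and player controller.
; DoUiCooldown starts cooldowns on primary UI slots matching this ability's class.
; IsCostStillAvailable checks that the Health, Mana or Strength attribute selected by the ability info's cost type strictly exceeds its cost.
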(event Ability|EventActivateAbility)

(event Ability|EventOnEndAbility
  (params (bWasCancelled :type Boolean)))

(fn GetPlayerInfo
  (bind _asbp_character_base (Utilities|Casting|CastToBP_CharacterBase (Ability|GetOwningActorfromActorInfo)))
  (bind _asbp_player_controller_base (Utilities|Casting|CastToBP_PlayerControllerBase (Pawn|GetController _asbp_character_base)))
  (return _asbp_character_base _asbp_player_controller_base))

(fn DoUiCooldown
  (bind _playercontrollerbase (CallFunction|GetPlayerInfo))
  (Utilities|IsValid _playercontrollerbase
    (:Is%20Valid
      (for _array_element (Variables|/Game/_Game/UI/PrimaryUI.PrimaryUI_C|GetSlots (Variables|/Game/_Game/Gameplay/BP_PlayerControllerBase.BP_PlayerControllerBase_C|GetPrimaryUI _playercontrollerbase))
        (bind _returnvalue (Class|GameplayAbilityBase|GetAbilityInfo))
        (if (== (.abilityclass (Variables|/Game/_Game/UI/WBP_AbilitySlot.WBP_AbilitySlot_C|GetAbility%20Info _array_element)) (.AbilityClass (Utilities|Struct|BreakGameplayAbilityInfo _returnvalue)))
          (Default|StartCoolDown _array_element))))))

(fn IsCostStillAvailable
  (bind _returnvalue (Class|GameplayAbilityBase|GetAbilityInfo))
  (LocalVariables|SetCost (.cost _returnvalue))
  (bind _characterbase (CallFunction|GetPlayerInfo))
  (Variables|Default|SetAttribute%20Set%20Base (Variables|/Script/AbilitySystem.CharacterBase|GetAttributeSetBase _characterbase))
  (switch Utilities|FlowControl|Switch|SwitchonEAbilityCostType (.costtype _returnvalue)
    (:Health
      (return (> (.currentvalue (Variables|/Script/AbilitySystem.AttributeSetBase|GetHealth (Variables|Default|GetAttribute%20Set%20Base))) (LocalVariables|GetCost))))
    (:Mana
      (return (> (.currentvalue (Variables|/Script/AbilitySystem.AttributeSetBase|GetMana (Variables|Default|GetAttribute%20Set%20Base))) (LocalVariables|GetCost))))
    (:Strength
      (return (> (.currentvalue (Variables|/Script/AbilitySystem.AttributeSetBase|GetStrength (Variables|Default|GetAttribute%20Set%20Base))) (LocalVariables|GetCost))))))