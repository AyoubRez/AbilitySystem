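; GA_Dash is a gameplay ability that dashes the character forward and damages, pushes and stuns characters reported as hit.
; On activation it commits, starts the UI cooldown, zeroes ground friction, applies a forward velocity impulse, sets pawn collision to overlap and plays the dash montage.
; Dash damage gameplay events supply targets for the damage effect and a knockback away from the owner.
; When the montage ends or is interrupted, friction and collision are restored.
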(event Ability|EventActivateAbility
  (Ability|CommitAbility)
  (CallFunction|DoUiCooldown)
  (bind _asbp_character_base (Utilities|Casting|CastToBP_CharacterBase (Ability|GetOwningActorfromActorInfo))
    (:then
      (Variables|Default|SetOriginal%20Ground%20Friction (Variables|/Script/Engine.CharacterMovementComponent|GetGroundFriction (Variables|/Script/Engine.Character|GetCharacterMovement _asbp_character_base)))
      (Variables|/Script/Engine.CharacterMovementComponent|SetGroundFriction (Variables|/Script/Engine.Character|GetCharacterMovement _asbp_character_base) 0.0)
      (Physics|AddImpulse (Variables|/Script/Engine.Character|GetCharacterMovement _asbp_character_base) (* (Transformation|GetActorForwardVector _asbp_character_base) 2e+03) true)
      (bind _characterbase (CallFunction|GetPlayerInfo))
      (Default|SetCollisiontopawn _characterbase "ECR_Overlap")
      (|PlayMontageandWaitProxy "None" "/Game/_Game/Character/Animations/AnimMontage/AM_Dash.AM_Dash" 1.0 "None" true 1.0 0.0
        (:then
          (bind _payload (Ability|Tasks|WaitGameplayEvent "(TagName=\"skill.dash.dealdamage\")" 0)
            (:EventReceived
              (GameplayEffects|ApplyGameplayEffectToTarget (Ability|TargetData|AbilityTargetDatafromActor (.Target (Utilities|Struct|BreakGameplayEventData _payload))) "/Game/_Game/Character/GameplayAbilities/Dash/GE_Dash_Damage.GE_Dash_Damage_C" 1 1)
              (bind _asbp_character_base_2 (Utilities|Casting|CastToBP_CharacterBase (.Target (Utilities|Struct|BreakGameplayEventData _payload))))
              (Default|PushCharacter _asbp_character_base_2 (Math|Vector|Normalize (- (Transformation|GetActorLocation _asbp_character_base_2) (Transformation|GetActorLocation (Ability|GetOwningActorfromActorInfo)))) 4e+03 5.0))))
        (:OnCompleted
          (Variables|/Script/Engine.CharacterMovementComponent|SetGroundFriction (Variables|/Script/Engine.Character|GetCharacterMovement _asbp_character_base) (Variables|Default|GetOriginal%20Ground%20Friction) :!label _label)
          (Default|SetCollisiontopawn _characterbase "ECR_Block")
          (Ability|EndAbility))
        (:OnBlendOut
          (goto _label))
        (:OnInterrupted
          (goto _label))
        (:OnCancelled
          (goto _label))))
    (:CastFailed
      (Ability|EndAbility))))

(event Ability|EventOnEndAbility
  (params (bWasCancelled :type Boolean)))