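; BP_Enemy is an enemy actor that continually turns to face the player.
; On BeginPlay it casts player character 0 to BP_CharacterBase and caches the reference.
; Each tick, a FacePlayer event interpolates toward the look-at rotation to that character and applies only the yaw, so the turn is smooth and stays horizontal.
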(event Custom|FacePlayer
  ;[1 1 1] Face player
  (Transformation|SetActorRotation (Math|Rotator|MakeRotator 0.0 0.0 (.yaw (Math|Interpolation|RInterpTo (Transformation|GetActorRotation) (Math|Rotator|FindLookatRotation (Transformation|GetActorLocation) (Transformation|GetActorLocation (Variables|Default|GetCharacter%20reference))) (Utilities|Time|GetWorldDeltaSeconds) 5.0)))))

(event EventBeginPlay
  (|CallParentFunction)
  (Utilities|FlowControl|Sequence
    (:then_0
      (bind _asbp_character_base (Utilities|Casting|CastToBP_CharacterBase (Game|GetPlayerCharacter 0)))
      (Variables|Default|SetCharacter%20reference _asbp_character_base))))

(event Collision|EventActorBeginOverlap
  (params (OtherActor :type Actor%20Object%20Reference))
  (|CallParentFunction OtherActor) ; This node is disabled and will not be called.\nDrag off pins to build functionality.
)

(event EventTick
  (params (DeltaSeconds :type Float%20%28single-precision%29))
  (|CallParentFunction DeltaSeconds)
  (CallFunction|FacePlayer))

(fn ConstructionScript
  (|CallParentFunction))