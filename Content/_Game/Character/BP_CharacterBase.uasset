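; BP_CharacterBase is a base character Blueprint built on the Gameplay Ability System, handling combat, health display and death.
; It grants initial abilities on BeginPlay and activates GA_Melee for attacks.
; Melee box and capsule overlaps send melee and dash damage gameplay events for hostile targets, with an exclude list preventing repeat dash hits.
; It also updates the health bar, toggles camera-driven rotation, applies low-friction knockback with stun, and prints Health every tick.
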(event OnComponentBeginOverlap(SwordCollider)
  (params (OverlappedComponent :type Primitive%20Component%20Object%20Reference) (OtherActor :type Actor%20Object%20Reference) (OtherComp :type Primitive%20Component%20Object%20Reference) (OtherBodyIndex :type Integer) (bFromSweep :type Boolean) (SweepResult :type Hit%20Result%20Structure%20%28by%20ref%29)))

(event OnComponentBeginOverlap(MeleeCollisionBox)
  (params (OverlappedComponent :type Primitive%20Component%20Object%20Reference) (OtherActor :type Actor%20Object%20Reference) (OtherComp :type Primitive%20Component%20Object%20Reference) (OtherBodyIndex :type Integer) (bFromSweep :type Boolean) (SweepResult :type Hit%20Result%20Structure%20%28by%20ref%29))
  (if (Actor|ActorHasTag OtherActor "Player")
    (bind _returnvalue (Class|CharacterBase|IsOtherHostile (.AsBP%20Character%20Base (Utilities|Casting|CastToBP_CharacterBase OtherActor))))
    (if _returnvalue
      (Ability|SendGameplayEventtoActor self "(TagName=\"skill.melee.dealdamage\")" (Utilities|Struct|MakeGameplayEventData "(TagName=\"\")" 0 OtherActor)))))

(event OnComponentBeginOverlap(CapsuleComponent)
  (params (OverlappedComponent :type Primitive%20Component%20Object%20Reference) (OtherActor :type Actor%20Object%20Reference) (OtherComp :type Primitive%20Component%20Object%20Reference) (OtherBodyIndex :type Integer) (bFromSweep :type Boolean) (SweepResult :type Hit%20Result%20Structure%20%28by%20ref%29))
  (bind _self self)
  (bind _asbp_character_base (Utilities|Casting|CastToBP_CharacterBase OtherActor))
  (bind _returnvalue (Class|CharacterBase|IsOtherHostile _asbp_character_base _self))
  (if _returnvalue
    (if (not (Utilities|Array|ContainsItem (Variables|Default|GetOverlapExclude) _asbp_character_base))
      (Utilities|Array|AddUnique (Variables|Default|GetOverlapExclude) _asbp_character_base)
      (Ability|SendGameplayEventtoActor self "(TagName=\"skill.dash.dealdamage\")" (Utilities|Struct|MakeGameplayEventData "(TagName=\"\")" _self OtherActor)))))

(event Custom|MeleeAttack
  (Abilities|TryActivateAbilitybyClass (Variables|Default|GetAbilitySystemComponent) "/Game/_Game/Character/GameplayAbilities/Melee/GA_Melee.GA_Melee_C" true))

(event Custom|PushCharacter
  (params (ImpulseDirection :type Vector) (PushStrength :type Float%20%28single-precision%29) (StunDuration :type Float%20%28single-precision%29))
  (bind _charactermovement (Variables|Character|GetCharacterMovement))
  (Variables|Default|SetGround%20Friction (Variables|/Script/Engine.CharacterMovementComponent|GetGroundFriction _charactermovement))
  (Variables|/Script/Engine.CharacterMovementComponent|SetGroundFriction _charactermovement 0.0)
  (Physics|AddImpulse _charactermovement (* ImpulseDirection PushStrength) true)
  (if (> StunDuration 0.0)
    (Class|CharacterBase|HitStun StunDuration))
  (Utilities|FlowControl|Delay 0.3)
  (Variables|/Script/Engine.CharacterMovementComponent|SetGroundFriction _charactermovement (Variables|Default|GetGround%20Friction)))

(event Custom|ClearOverlapExculde
  (Utilities|Array|Clear (Variables|Default|GetOverlapExclude)))

(event Custom|Stun)

(event Custom|MakeCameraControlRotation
  (params (ShouldControlRotation :type Boolean))
  (bind _charactermovement (Variables|Character|GetCharacterMovement))
  (if ShouldControlRotation
    (Variables|Default|SetbUseControllerRotationYaw true)
    (Variables|/Script/Engine.CharacterMovementComponent|SetbOrientRotationToMovement _charactermovement false)
    (else
      (Variables|Default|SetbUseControllerRotationYaw false)
      (Variables|/Script/Engine.CharacterMovementComponent|SetbOrientRotationToMovement _charactermovement true))))

(event EventBeginPlay
  (Class|CharacterBase|AcquireAbilities (Variables|Default|GetInitialAbilities)))

(event Collision|EventActorBeginOverlap
  (params (OtherActor :type Actor%20Object%20Reference)))

(event EventTick
  (params (DeltaSeconds :type Float%20%28single-precision%29))
  (Development|PrintString (Utilities|String|ToString(Float) (.currentvalue (Variables|/Script/AbilitySystem.AttributeSetBase|GetHealth (Variables|Default|GetAttributeSetBase)))) true true "(R=0.000000,G=0.660000,B=1.000000,A=1.000000)" 0.0))

(event EventOnHealthChange
  (params (Health :type Float%20%28single-precision%29) (MaxHealth :type Float%20%28single-precision%29))
  (bind _ashealth_bar (Utilities|Casting|CastToHealthBar (UserInterface|GetUserWidgetObject (Variables|Default|GetHealthBar))))
  (Default|SetPercentage _ashealth_bar (/ Health MaxHealth)))

(event EventDie
  (bind _returnvalue (Animation|PlayAnimMontage "/Game/_Game/Character/Animations/AnimMontage/DeathMontage.DeathMontage" 1.0 "None"))
  (Utilities|FlowControl|Delay _returnvalue)
  (Actor|DestroyActor))

(fn ConstructionScript)

(fn SetCollisiontopawn
  (params (response :type ECollisionResponse%20Enum :default "ECR_Overlap"))
  (Collision|SetCollisionResponsetoChannel (Variables|Default|GetCapsuleComponent) "ECC_Pawn" response))